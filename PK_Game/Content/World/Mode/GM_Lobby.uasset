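; GM_Lobby is the lobby game mode, which periodically refreshes a display through the game instance.
; Tick increments a counter and, on reaching five, casts the game instance to Kemijarvi, calls RefreshDisplay and resets the counter, so the refresh is throttled by frame count rather than time.
; An unconnected switch on the counter holds placeholder prints for pull, load, save and push data stages and never runs.
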(event EventBeginPlay)

(event EventTick
  (params (DeltaSeconds :type Float%20%28single-precision%29))
  (Math|Integer|IncrementInt (Variables|Default|GetTick_Timer)
    (:%20%20
      (if (>= (Variables|Default|GetTick_Timer) 5)
        (bind _askemijarvi (Utilities|Casting|CastToKemijarvi (Game|GetGameInstance)))
        (Default|RefreshDisplay _askemijarvi)
        (Variables|Default|SetTick_Timer 0)))))

(fn ConstructionScript)