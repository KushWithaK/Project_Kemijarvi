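; PC_User is a player controller that puts the player into the login or lobby screen at start.
; On BeginPlay it copies Username, Code and PlayerName from the Kemijarvi game instance, then runs FixPlayer to show the mouse cursor.
; When Code is "Offline", it opens AW_Login for an empty Username, otherwise SW_Lobby.
; Tick cycles a counter into a switch with no actions attached.
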(event EventBeginPlay
  (CallFunction|CallPlayer))

(event EventTick
  (params (DeltaSeconds :type Float%20%28single-precision%29))
  (Math|Integer|IncrementInt (Variables|Default|GetTick_Timer)
    (:%20%20
      (if (>= (Variables|Default|GetTick_Timer) 9)
        (Variables|Default|SetTick_Timer 0)
        (else
          (switch int (Variables|Default|GetTick_Timer)))))))

(fn ConstructionScript)

(fn CallPlayer
  (bind _askemijarvi (Utilities|Casting|CastToKemijarvi (Game|GetGameInstance)))
  (Variables|Default|SetUsername (Variables|/Game/World/Kemijarvi.Kemijarvi_C|GetUsername _askemijarvi))
  (Variables|Default|SetCode (Variables|/Game/World/Kemijarvi.Kemijarvi_C|GetCode _askemijarvi))
  (Variables|Default|SetPlayer_Name (Variables|/Game/World/Kemijarvi.Kemijarvi_C|GetPlayerName _askemijarvi))
  (Utilities|FixPlayer
    (:Out
      (return))))